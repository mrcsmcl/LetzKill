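; Actor that fetches sun and weather data from the HeliosTime web API for the game.
; On BeginPlay it sends an HTTP GET, then repeats the request on a looping 20-minute timer.
; A successful response is parsed as JSON; helper functions extract sun pitch and yaw plus sky and temperature.
; These values are stored in the HeliosTimeAPI struct on BP_GameInstance; failed requests are not handled.
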(event `self.ReceiveBeginPlay`
  (`KismetSystemLibrary.K2_SetTimerDelegate` (delegate `API Request Every 20min`) 1200.0 true)
  (bind (_outheader _result_body) (`|HttpRequest` (`self.HeliosTime API URL`) "Get" :!label _label)
    (:`On Success`
      (bind _outjsonobject (`JsonBlueprintFunctionLibrary.FromString` _result_body))
      (`KismetSystemLibrary.PrintString` "Conectado a Heliostime API")
      (set `self.Json Object` _outjsonobject)
      (bind _asbp_game_instance (cast `/Game/Main/BP_GameInstance` (`GameplayStatics.GetGameInstance`)))
      (set `self.As BP Game Instance` _asbp_game_instance)
      (bind _outvalue (`|GetJsonField` (`self.Json Object`) "weather"))
      (bind _outvalue_2 (`|GetJsonField` _outvalue "sky"))
      (bind _outvalue_3 (`|GetJsonField` _outvalue "temperature"))
      (bind _outvalue_4 (`|GetJsonField` (`self.Json Object`) "sun"))
      (bind _outvalue_5 (`|GetJsonField` _outvalue_4 "pitch"))
      (bind _outvalue_6 (`|GetJsonField` _outvalue_4 "yaw"))
      (set `/Game/Main/BP_GameInstance.HeliosTime API` (make `/Game/Main/APIs/S_HeliosTimeAPI` _outvalue_5 _outvalue_6 _outvalue_2 _outvalue_3) (`self.As BP Game Instance`)))))

(event `API Request Every 20min`
  (goto _label))

(fn `UserConstructionScript`)